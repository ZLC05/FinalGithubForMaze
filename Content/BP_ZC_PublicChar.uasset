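; Player character Blueprint that handles a limited-use area stun against enemies, the player HUD and pausing.
; BeginPlay adds the PlayerUI widget, which shows the remaining flashbang count, and hides the mouse cursor.
; The Stun input spends a charge, updates the HUD, then runs a multi-sphere object trace around the character and calls Stunned on BP_ZCEnemy hits.
; Escape or 0 opens the pause widget, pauses the game and shows the cursor.
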(event `self.ReceiveBeginPlay`
  ; Adding UI at the start of the game
  (bind _returnvalue (`|CreateWidget` "/Game/Widgets/PlayerUI.PlayerUI_C"))
  (set `self.flashbangUI` _returnvalue)
  (`UserWidget.AddToViewport` (`self.flashbangUI`) 0)
  (set `PlayerController.bShowMouseCursor` false (`GameplayStatics.GetPlayerController` 0)))

(event `InputAction|Stun`
  (params (Key :type "Key Structure"))
  ; Enemy Stunning
  (:`Pressed`
    (if (> (`self.StunAmounts`) 0)
      (`KismetSystemLibrary.PrintString` (`KismetStringLibrary.Conv_IntToString` (`self.StunAmounts`)))
      (bind _result (`/Engine/EditorBlueprintResources/StandardMacros.DecrementInt` (`self.StunAmounts`))
        (:`  `
          (bind _output_get (set `self.StunAmounts` _result))
          (`/Game/Widgets/PlayerUI.UpdateFlashbangValue` (`self.flashbangUI`) _output_get)
          (bind (_outhits _returnvalue) (`KismetSystemLibrary.SphereTraceMultiForObjects` (`self.K2_GetActorLocation`) (0.0 0.0 0.0) (`self.stunRadius`) (`self.stunObjectTypes`)))
          (if _returnvalue
            (for _array_element _outhits
              (bind _asbp_zcenemy (cast `/Game/AI/BP_ZCEnemy` (`.HitActor` (`GameplayStatics.BreakHitResult` _array_element))))
              (`/Game/AI/BP_ZCEnemy.Stunned` _asbp_zcenemy)))))
      (else
        (`KismetSystemLibrary.PrintString` "No more sutns")))))

(event `Key|Escape`
  (params (Key :type "Key Structure"))
  (bind _returnvalue (`GameplayStatics.GetPlayerController` 0))
  ; Activates The Keyboard Event for Pausing the game
  (:`Pressed`
    (bind _returnvalue_2 (`|CreateWidget` "/Game/Widgets/PauseWidgetBP1.PauseWidgetBP1_C" _returnvalue))
    (`UserWidget.AddToViewport` _returnvalue_2 0)
    (`GameplayStatics.SetGamePaused` true)
    (set `PlayerController.bShowMouseCursor` true _returnvalue)))

(event `Key|Zero`
  (params (Key :type "Key Structure"))
  (bind _returnvalue (`GameplayStatics.GetPlayerController` 0))
  ; Activates The Keyboard Event for Pausing the game
  (:`Pressed`
    (bind _returnvalue_2 (`|CreateWidget` "/Game/Widgets/PauseWidgetBP1.PauseWidgetBP1_C" _returnvalue))
    (`UserWidget.AddToViewport` _returnvalue_2 0)
    (`GameplayStatics.SetGamePaused` true)
    (set `PlayerController.bShowMouseCursor` true _returnvalue)))

(fn `UserConstructionScript`)